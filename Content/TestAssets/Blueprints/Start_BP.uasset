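; Grabbable physics actor that opens the "Beta" level when its Hit event fires, apparently serving as a start object.
; Pickup turns off mesh physics and attaches the actor to the given component; Drop restores physics and detaches it.
; Tick destroys the actor after a few seconds unless it is grabbed; Drop never clears Grabbed, so one pickup permanently stops that timer.
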(event Collision|EventHit
  (params (MyComp :type Primitive%20Component%20Object%20Reference) (Other :type Actor%20Object%20Reference) (OtherComp :type Primitive%20Component%20Object%20Reference) (bSelfMoved :type Boolean) (HitLocation :type Vector :default "0, 0, 0") (HitNormal :type Vector :default "0, 0, 0") (NormalImpulse :type Vector :default "0, 0, 0") (Hit :type Hit%20Result%20Structure%20%28by%20ref%29))
  ;[1 1 1] Change Level
  (Game|OpenLevel(byName) "Beta"))

(event EventTick
  (params (DeltaSeconds :type Float%20%28single-precision%29))
  ;[1 1 1] Destroy
  (if (not (Variables|Default|GetGrabbed))
    (bind _output_get (Variables|Default|SetCounter (+ DeltaSeconds (Variables|Default|GetCounter))))
    (if (>= _output_get 5.0)
      (Actor|DestroyActor))))

(event EventPickup
  (params (Attach%20To :type Scene%20Component%20Object%20Reference))
  ;[1 1 1] Pickup and Drop
  (Physics|SetSimulatePhysics (Variables|Default|GetStaticMesh) false)
  (Transformation|AttachComponentToComponent (Variables|Transformation|GetRootComponent) Attach%20To "None" "KeepWorld" "KeepWorld" "KeepWorld" true)
  (Variables|Default|SetGrabbed true)
  (Variables|Default|SetCounter 0.0))

(event EventDrop
  ;[1 1 1] Pickup and Drop
  (Physics|SetSimulatePhysics (Variables|Default|GetStaticMesh) true)
  (Transformation|DetachFromActor "KeepWorld" "KeepWorld" "KeepWorld"))

(fn ConstructionScript)