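; A repeating geyser that alternates between dormant and erupting every few seconds and launches objects that enter it.
; Tick drives a counter that toggles the smoke effect and the ImpulseVolume's overlap events, which apply a delayed, mass-scaled impulse to non-boulders.
; A Boulder_Temp in BoulderVolume blocks the geyser; if still blocked after a delay, it gets launched with added BoulderVelocity and an eruption begins.
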(event OnComponentBeginOverlap(ImpulseVolume)
  (params (OverlappedComponent :type Primitive%20Component%20Object%20Reference) (OtherActor :type Actor%20Object%20Reference) (OtherComp :type Primitive%20Component%20Object%20Reference) (OtherBodyIndex :type Integer) (bFromSweep :type Boolean) (SweepResult :type Hit%20Result%20Structure%20%28by%20ref%29))
  ;[1 1 1] Launch non-Boulders
  (Utilities|Casting|CastToBoulder_Temp OtherActor
    (:CastFailed
      (Utilities|FlowControl|Delay 0.1)
      (bind _asprimitive_component (Utilities|Casting|CastToPrimitiveComponent (Variables|/Script/Engine.Actor|GetRootComponent OtherActor)))
      (Physics|AddImpulseatLocation _asprimitive_component (* (Variables|Default|GetImpulseMultiplier) (Physics|GetMass _asprimitive_component)) (Transformation|GetWorldLocation _asprimitive_component) "None"))))

(event OnComponentBeginOverlap(BoulderVolume)
  (params (OverlappedComponent :type Primitive%20Component%20Object%20Reference) (OtherActor :type Actor%20Object%20Reference) (OtherComp :type Primitive%20Component%20Object%20Reference) (OtherBodyIndex :type Integer) (bFromSweep :type Boolean) (SweepResult :type Hit%20Result%20Structure%20%28by%20ref%29))
  ;[1 1 1] Handle Boulders
  (bind _asboulder_temp (Utilities|Casting|CastToBoulder_Temp OtherActor))
  (bind _output_get (Variables|Default|SetIsBlocked true))
  (Utilities|FlowControl|Delay 6.0)
  (if _output_get
    (bind _asprimitive_component (Utilities|Casting|CastToPrimitiveComponent (Variables|/Script/Engine.Actor|GetRootComponent _asboulder_temp)))
    (Physics|AddImpulseatLocation _asprimitive_component (+ (* (Variables|Default|GetImpulseMultiplier) (Physics|GetMass _asprimitive_component)) (* (Variables|/Game/TestAssets/Blueprints/Boulder_Temp.Boulder_Temp_C|GetBoulder%20Velocity _asboulder_temp) 1000)) (Transformation|GetWorldLocation _asprimitive_component) "None")
    (Variables|Default|SetIsBlocked false)
    (Variables|Default|SetCounter 3.0)))

(event OnComponentEndOverlap(BoulderVolume)
  (params (OverlappedComponent :type Primitive%20Component%20Object%20Reference) (OtherActor :type Actor%20Object%20Reference) (OtherComp :type Primitive%20Component%20Object%20Reference) (OtherBodyIndex :type Integer))
  ;[1 1 1] Handle Boulders
  (Utilities|Casting|CastToBoulder_Temp OtherActor)
  (Variables|Default|SetIsBlocked false))

(event EventTick
  (params (DeltaSeconds :type Float%20%28single-precision%29))
  ;[1 1 1] Alternate Geyser Activity
  (if (Variables|Default|GetIsBlocked)
    (Components|Activation|Deactivate (Variables|Default|GetGeyser_Smoke))
    (Variables|/Script/Engine.PrimitiveComponent|SetbGenerateOverlapEvents (Variables|Default|GetImpulseVolume) false)
    (else
      (Variables|Default|SetCounter (+ DeltaSeconds (Variables|Default|GetCounter)))
      (if (>= (Variables|Default|GetCounter) 3.0)
        (Components|Activation|Activate (Variables|Default|GetGeyser_Smoke) false)
        (Variables|/Script/Engine.PrimitiveComponent|SetbGenerateOverlapEvents (Variables|Default|GetImpulseVolume) true)
        (if (>= (Variables|Default|GetCounter) 6.0)
          (Components|Activation|Deactivate (Variables|Default|GetGeyser_Smoke))
          (Variables|/Script/Engine.PrimitiveComponent|SetbGenerateOverlapEvents (Variables|Default|GetImpulseVolume) false)
          (Variables|Default|SetCounter 0.0))))))

(event EventBeginPlay
  ;[1 1 1] Start with Geyser Off
  (Components|Activation|Deactivate (Variables|Default|GetGeyser_Smoke))
  (Variables|/Script/Engine.PrimitiveComponent|SetbGenerateOverlapEvents (Variables|Default|GetImpulseVolume) false))

(fn ConstructionScript)