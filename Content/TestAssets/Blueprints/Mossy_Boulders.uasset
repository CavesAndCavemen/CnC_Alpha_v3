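; Mossy boulder pickup that players can carry and drop, and that turns into a BP_DeadIsland when clustered with other boulders.
; Pickup and Drop toggle sphere physics and attachment.
; Tick waits for near-zero velocity, then spawns the island if a box overlap finds exactly three boulders, using the river actor's height, and destroys them.
; The DidNotSpawn flag blocks retries until the boulder moves again.
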(event EventPickup
  (params (Attach%20To :type Scene%20Component%20Object%20Reference))
  ;[1 1 1] Pickup and Drop
  (Physics|SetSimulatePhysics (Variables|Default|GetSphere) false)
  (Transformation|AttachComponentToComponent (Variables|Transformation|GetRootComponent) Attach%20To "None" "KeepWorld" "KeepWorld" "KeepWorld" true))

(event EventDrop
  ;[1 1 1] Pickup and Drop
  (Physics|SetSimulatePhysics (Variables|Default|GetSphere) true)
  (Transformation|DetachFromActor "KeepWorld" "KeepWorld" "KeepWorld"))

(event EventTick
  (params (DeltaSeconds :type Float%20%28single-precision%29))
  (bind _self self)
  (bind _returnvalue (Transformation|GetActorLocation _self))
  (bind (_x _y) (Math|Vector|BreakVector _returnvalue))
  ;[1 1 1] Spawn Mossy Islands
  ;;[1 1 1] Check if Moving
  (if (Math|Vector|Equal(Vector) (Transformation|GetVelocity self) "0, 0, 0" 1.0)
    ;;[1 1 1] If not Moving, Check for Two Mossy Boulders
    (bind _outactors (Collision|BoxOverlapActors (Transformation|GetActorLocation self) "100.000000,100.000000,100.000000" (Utilities|Array|MakeArray "ObjectTypeQuery4") "Mossy_Boulders_C" :!class /Script/Engine.KismetSystemLibrary))
    ;;[1 1 1] Spawn Island and Destroy Mossy Boulders
    (if (and (== (Utilities|Array|Length _outactors) 3) (not (Variables|Default|GetDid%20Not%20Spawn)))
      (bind _outactors_2 (Collision|BoxOverlapActors _returnvalue "10.000000,10.000000,50.000000" (Utilities|Array|MakeArray "ObjectTypeQuery1") "/Game/TestAssets/Blueprints/River_Temp_BP.River_Temp_BP_C" :!class /Script/Engine.KismetSystemLibrary))
      (Game|SpawnActorfromClass "/Game/TestAssets/Blueprints/BP_DeadIsland.BP_DeadIsland_C" (Math|Transform|MakeTransform (Math|Vector|MakeVector _x _y (+ (.Z (Math|Vector|BreakVector (Transformation|GetActorLocation (Utilities|Array|Get(acopy) _outactors_2)))) 5.0))) "Undefined" 0 0)
      (for _array_element _outactors
        (Actor|DestroyActor _array_element))
      (Actor|DestroyActor)
      (else
        ;;[1 1 1] Ignore Two MBs when Spawning Islands
        (Variables|Default|SetDid%20Not%20Spawn true)))
    (else
      (Variables|Default|SetDid%20Not%20Spawn false))))

(fn ConstructionScript)