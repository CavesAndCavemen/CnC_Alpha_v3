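; Tree actor that grows BP_Telefruit pickups and replaces them when picked.
; On BeginPlay it spawns a fruit at each of its marker scene components, storing the spawn transform, disabling mesh physics so it hangs, and passing itself as HomeTree.
; The FruitPicked event, given a location, spawns and initializes a replacement fruit there the same way.
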(event Custom|FruitPicked
  (params (Location :type Transform))
  ;[1 1 1] Spawn New Fruit
  (bind _returnvalue (Game|SpawnActorfromClass "/Game/TestAssets/Blueprints/BP_Telefruit.BP_Telefruit_C" Location "Undefined" 0 0))
  (Variables|/Game/TestAssets/Blueprints/BP_Telefruit.BP_Telefruit_C|SetSpawn%20Location _returnvalue (Math|Conversions|ToTransform(Vector) (Transformation|GetWorldLocation (Variables|/Script/Engine.Actor|GetRootComponent _returnvalue))))
  (Physics|SetSimulatePhysics (Variables|/Script/Engine.StaticMeshActor|GetStaticMeshComponent _returnvalue) false)
  (Variables|/Game/TestAssets/Blueprints/BP_Telefruit.BP_Telefruit_C|SetHomeTree _returnvalue self))

(event EventBeginPlay
  ;[1 1 1] Spawn Fruit
  (for _array_element (Utilities|Array|MakeArray (Variables|Default|GetScene1) (Variables|Default|GetScene2) (Variables|Default|GetScene3) (Variables|Default|GetScene4) (Variables|Default|GetScene5) (Variables|Default|GetScene6) (Variables|Default|GetScene7) (Variables|Default|GetScene))
    (bind _returnvalue (Game|SpawnActorfromClass "/Game/TestAssets/Blueprints/BP_Telefruit.BP_Telefruit_C" (Math|Conversions|ToTransform(Vector) (Transformation|GetWorldLocation _array_element)) "Undefined" 0 0))
    (Variables|/Game/TestAssets/Blueprints/BP_Telefruit.BP_Telefruit_C|SetSpawn%20Location _returnvalue (Math|Conversions|ToTransform(Vector) (Transformation|GetWorldLocation (Variables|/Script/Engine.Actor|GetRootComponent _returnvalue))))
    (Physics|SetSimulatePhysics (Variables|/Script/Engine.StaticMeshActor|GetStaticMeshComponent _returnvalue) false)
    (Variables|/Game/TestAssets/Blueprints/BP_Telefruit.BP_Telefruit_C|SetHomeTree _returnvalue self)))

(fn ConstructionScript)