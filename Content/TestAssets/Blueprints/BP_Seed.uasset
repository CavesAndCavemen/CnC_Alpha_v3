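; A grabbable seed fruit that turns dead islands into forested ones.
; Pickup attaches it and, after a short delay, tells its home SeedTree it was picked; Drop detaches it and restores physics.
; Hitting an unforested BP_DeadIsland after pickup spawns a tree, applies grass and destroys the seed.
; Other hits or river overlaps can start a timeout that destroys it once it is simulating physics away from the player.
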(event Collision|EventActorBeginOverlap
  (params (OtherActor :type Actor%20Object%20Reference))
  ;[1 1 1] If Land in River,  Test Destroy
  (Utilities|Casting|CastToRiver_Temp_BP OtherActor)
  (Variables|Default|SetIsGrabbed false)
  (Variables|Default|SetTest%20for%20Destroy true))

(event EventPickup
  (params (Attach%20To :type Scene%20Component%20Object%20Reference))
  ;[1 1 1] Pickup and Drop
  (Physics|SetSimulatePhysics (Variables|Debug|GetStaticMeshComponent) false)
  (bind _returnvalue (Transformation|AttachComponentToComponent (VehicleSound|GetRootComponent) Attach%20To "None" "KeepWorld" "KeepWorld" "KeepWorld" false))
  (Variables|Default|SetIsGrabbed _returnvalue)
  (Variables|Default|SetTest%20for%20Destroy false)
  (Variables|Default|SetDestructionCounter 0.0)
  ;[1 1 1] Spawn New Fruit
  (Utilities|FlowControl|Delay 3.0)
  (bind _asseed_tree (Utilities|Casting|CastToSeedTree (Variables|Default|GetHomeTree)))
  (Default|FruitPicked _asseed_tree (Variables|Default|GetSpawn%20Location) self))

(event EventDrop
  ;[1 1 1] Pickup and Drop
  (Physics|SetSimulatePhysics (Variables|Debug|GetStaticMeshComponent) true)
  (Transformation|DetachFromActor "KeepWorld" "KeepWorld" "KeepWorld"))

(event Collision|EventHit
  (params (MyComp :type Primitive%20Component%20Object%20Reference) (Other :type Actor%20Object%20Reference) (OtherComp :type Primitive%20Component%20Object%20Reference) (bSelfMoved :type Boolean) (HitLocation :type Vector :default "0, 0, 0") (HitNormal :type Vector :default "0, 0, 0") (NormalImpulse :type Vector :default "0, 0, 0") (Hit :type Hit%20Result%20Structure%20%28by%20ref%29))
  ;[1 1 1] Fertilize Dead Island
  (if (Variables|Default|GetIsGrabbed)
    (bind _asbp_dead_island (Utilities|Casting|CastToBP_DeadIsland Other)
      (:then
        (if (Variables|/Game/TestAssets/Blueprints/BP_DeadIsland.BP_DeadIsland_C|GetIsForested _asbp_dead_island)
          (Variables|Default|SetTest%20for%20Destroy true :!label _label)
          (else
            (Game|SpawnActorfromClass "/Game/TestAssets/Blueprints/Tree.Tree_C" (Math|Transform|MakeTransform (+ (Transformation|GetActorLocation _asbp_dead_island) "0,0.000000,35.000000")) "Undefined" 0 0)
            (Variables|/Game/TestAssets/Blueprints/BP_DeadIsland.BP_DeadIsland_C|SetIsForested _asbp_dead_island true)
            (Rendering|Material|SetMaterial (Variables|/Game/TestAssets/Blueprints/BP_Floor.BP_Floor_C|GetIsland _asbp_dead_island) 0 "/Game/TestAssets/Materials/grass_mat.grass_mat")
            (Utilities|FlowControl|Delay 0.05)
            (Actor|DestroyActor))))
      (:CastFailed
        (goto _label)))
    (elif (!= (Variables|Default|GetHomeTree) 0)
      (goto _label))))

(event EventTick
  (params (DeltaSeconds :type Float%20%28single-precision%29))
  ;[1 1 1] Destroy if Unnecessary
  (if (Variables|Default|GetTest%20for%20Destroy)
    (bind _output_get (Variables|Default|SetDestructionCounter (+ DeltaSeconds (Variables|Default|GetDestructionCounter))))
    (if (Math|Boolean|ANDBoolean (>= _output_get 1.2e+02) (Physics|IsSimulatingPhysics (Variables|Debug|GetStaticMeshComponent) "None") (Math|Vector|NotEqual(Vector) (Transformation|GetActorLocation) (Transformation|GetActorLocation (Game|Player|GetPlayerPawn 0)) 1.5e+02))
      (Actor|DestroyActor))))

(fn ConstructionScript)