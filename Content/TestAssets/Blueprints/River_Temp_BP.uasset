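; Temporary river actor that floats telefruits, boulders and mossy boulders and pushes them along a current set by its yaw at BeginPlay.
; Each tick it loops over tracked overlapping actors, applying upward force inside the Underwater component and current force while horizontal speed is at or below a cap.
; Forces on root components vary by each object's RiverName.
; The entry velocity-cancelling impulse is disconnected and never runs.
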(event OnComponentBeginOverlap(Underwater)
  (params (OverlappedComponent :type Primitive%20Component%20Object%20Reference) (OtherActor :type Actor%20Object%20Reference) (OtherComp :type Primitive%20Component%20Object%20Reference) (OtherBodyIndex :type Integer) (bFromSweep :type Boolean) (SweepResult :type Hit%20Result%20Structure%20%28by%20ref%29))
  ;[1 1 1] Upon First Entry, Negate Velocity
)

(event EventBeginPlay
  (bind _returnvalue (Transformation|GetActorRotation))
  (bind _yaw (Math|Rotator|BreakRotator _returnvalue))
  ;[1 1 1] Set Current Direction
  (Variables|Default|SetCurrentDirection (Math|Vector|MakeVector (Math|Trig|Cos(Degrees) _yaw) (Math|Trig|Sin(Degrees) _yaw) 0.0)))

(event Collision|EventActorBeginOverlap
  (params (OtherActor :type Actor%20Object%20Reference))
  ;[1 1 1] Overlapping are Effected
  (Utilities|Array|Add (Variables|Default|GetOverlappingActors) OtherActor))

(event Collision|EventActorEndOverlap
  (params (OtherActor :type Actor%20Object%20Reference))
  ;[1 1 1] No-longer Overlapping are Uneffected
  (Utilities|Array|RemoveItem (Variables|Default|GetOverlappingActors) OtherActor))

(event EventTick
  (params (DeltaSeconds :type Float%20%28single-precision%29))
  ;[1 1 1] If Any Overlap, Push with Current
  (if (>= (Utilities|Array|Length (Variables|Default|GetOverlappingActors)) 1)
    (for _array_element (Variables|Default|GetOverlappingActors)
      (bind _objectname (CallFunction|GetObjectName _array_element))
      (bind _asprimitive_component (Utilities|Casting|CastToPrimitiveComponent (Variables|/Script/Engine.Actor|GetRootComponent _array_element)))
      (Utilities|FlowControl|Sequence
        (:then_0
          (if (Collision|IsOverlappingActor (Variables|Default|GetUnderwater) _array_element :!class /Script/Engine.PrimitiveComponent)
            (CallFunction|AddVerticalForce _asprimitive_component _objectname)))
        (:then_1
          (if (<= (Class|KismetMathLibrary|Hypotenuse (Math|Float|Absolute(Float) (.X (Math|Vector|BreakVector (Transformation|GetVelocity _array_element)))) (Math|Float|Absolute(Float) (.Y (Math|Vector|BreakVector (Transformation|GetVelocity _array_element))))) 1.5e+02)
            (CallFunction|AddHorizontalForce _asprimitive_component _objectname)))))))

(fn ConstructionScript)

(fn GetObjectName
  (params (Object :type Actor%20Object%20Reference))
  (bind _asbp_telefruit (Utilities|Casting|CastToBP_Telefruit Object)
    (:then
      (LocalVariables|SetName (Variables|/Game/TestAssets/Blueprints/BP_Telefruit.BP_Telefruit_C|GetRiverName _asbp_telefruit)))
    (:CastFailed
      (bind _asboulder_temp (Utilities|Casting|CastToBoulder_Temp Object)
        (:then
          (LocalVariables|SetName (Variables|/Game/TestAssets/Blueprints/Boulder_Temp.Boulder_Temp_C|GetRiverName _asboulder_temp)))
        (:CastFailed
          (bind _asmossy_boulders (Utilities|Casting|CastToMossy_Boulders Object))
          (LocalVariables|SetName (Variables|/Game/TestAssets/Blueprints/Mossy_Boulders.Mossy_Boulders_C|GetRiverName _asmossy_boulders))))))
  (return (LocalVariables|GetName)))

(fn AddVerticalForce
  (params (Primitive%20Component :type Primitive%20Component%20Object%20Reference) (ObjectName :type Name))
  (switch name ObjectName
    (:Telefruit
      (Physics|AddForce Primitive%20Component "0, 0,150000.000000" "None" false))
    (:MossyBoulder
      (Physics|AddForce Primitive%20Component "0, 0,325000.000000" "None" false))
    (:Boulder
      (Physics|AddForce Primitive%20Component "0, 0,750000.000000" "None" false))))

(fn AddHorizontalForce
  (params (Primitive%20Component :type Primitive%20Component%20Object%20Reference) (ObjectName :type Name))
  (bind _currentdirection (Variables|Default|GetCurrentDirection))
  (switch name ObjectName
    (:Telefruit
      (Physics|AddForce Primitive%20Component (* (LocalVariables|GetTelefruit%20Force) _currentdirection) "None" false))
    (:MossyBoulder
      (Physics|AddForce Primitive%20Component (* (LocalVariables|GetMossyBoulder%20Force) _currentdirection) "None" false))
    (:Boulder
      (Physics|AddForce Primitive%20Component (* _currentdirection (LocalVariables|GetBoulder%20Force)) "None" false))))