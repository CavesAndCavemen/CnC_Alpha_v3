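; Seed tree actor that carries BP_Seed fruit, drops it when struck by a moving boulder and regrows it.
; On BeginPlay it spawns non-simulating, distance-culled seeds at six scene component points, each storing its spawn transform and home tree.
; A Boulder_Temp hit above a velocity tolerance enables physics on carried seeds, then respawns the full set after a short delay.
; FruitPicked removes the picked seed and immediately spawns a replacement at the given location.
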(event Custom|FruitPicked
  (params (Location :type Transform) (Picked%20Fruit :type Actor%20Object%20Reference))
  ;[1 1 1] Spawn Fruit when Picked
  (Utilities|Array|RemoveItem (Variables|Default|GetCarried%20Fruit) Picked%20Fruit)
  (CallFunction|SpawnSeed Location))

(event EventBeginPlay
  ;[1 1 1] Spawn All Fruit
  (for _array_element (Utilities|Array|MakeArray (Variables|Default|GetScene1) (Variables|Default|GetScene2) (Variables|Default|GetScene3) (Variables|Default|GetScene4) (Variables|Default|GetScene5) (Variables|Default|GetScene))
    (CallFunction|SpawnSeed (Math|Conversions|ToTransform(Vector) (Transformation|GetWorldLocation _array_element)))))

(event Collision|EventHit
  (params (MyComp :type Primitive%20Component%20Object%20Reference) (Other :type Actor%20Object%20Reference) (OtherComp :type Primitive%20Component%20Object%20Reference) (bSelfMoved :type Boolean) (HitLocation :type Vector :default "0, 0, 0") (HitNormal :type Vector :default "0, 0, 0") (NormalImpulse :type Vector :default "0, 0, 0") (Hit :type Hit%20Result%20Structure%20%28by%20ref%29))
  (bind _carried_fruit (Variables|Default|GetCarried%20Fruit))
  ;[1 1 1] Drop All Seeds when Hit
  (bind _asboulder_temp (Utilities|Casting|CastToBoulder_Temp Other))
  (if (Math|Vector|NotEqual(Vector) (Transformation|GetVelocity _asboulder_temp) "0, 0, 0" 5e+01)
    (Utilities|FlowControl|Sequence
      (:then_0
        (for _array_element _carried_fruit
          (bind _asbp_seed (Utilities|Casting|CastToBP_Seed _array_element))
          (Physics|SetSimulatePhysics (Variables|/Script/Engine.StaticMeshActor|GetStaticMeshComponent _asbp_seed) true)
          (Utilities|Array|RemoveItem _carried_fruit _array_element)))
      (:then_1
        (Utilities|FlowControl|Delay 3.0)
        ;[1 1 1] Spawn All Fruit
        (for _array_element_2 (Utilities|Array|MakeArray (Variables|Default|GetScene1) (Variables|Default|GetScene2) (Variables|Default|GetScene3) (Variables|Default|GetScene4) (Variables|Default|GetScene5) (Variables|Default|GetScene))
          (CallFunction|SpawnSeed (Math|Conversions|ToTransform(Vector) (Transformation|GetWorldLocation _array_element_2))))))))

(fn ConstructionScript)

(fn SpawnSeed
  (params (NewParam :type Transform))
  (bind _returnvalue (Game|SpawnActorfromClass "/Game/TestAssets/Blueprints/BP_Seed.BP_Seed_C" NewParam "Undefined" 0 0))
  (Class|PrimitiveComponent|SetCullDistance (Variables|/Script/Engine.StaticMeshActor|GetStaticMeshComponent _returnvalue) 3e+03)
  (Variables|/Game/TestAssets/Blueprints/BP_Seed.BP_Seed_C|SetSpawn%20Location _returnvalue NewParam)
  (Physics|SetSimulatePhysics (Variables|/Script/Engine.StaticMeshActor|GetStaticMeshComponent _returnvalue) false)
  (Variables|/Game/TestAssets/Blueprints/BP_Seed.BP_Seed_C|SetHomeTree _returnvalue self)
  (Utilities|Array|Add (Variables|Default|GetCarried%20Fruit) _returnvalue))