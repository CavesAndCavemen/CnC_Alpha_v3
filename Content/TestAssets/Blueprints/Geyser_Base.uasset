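; Base geyser actor that cycles on a Tick-driven timer through idle, small geyser and smoke eruption phases.
; On BeginPlay it spawns and attaches a hidden BouncePad, whose overlap events switch on with the small geyser and off when the cycle resets.
; During the smoke phase a collision BlockBox rises into place, then drops away at reset.
; A Boulder_Temp detected by a box overlap pauses the timer and disables smoke, blocking and bouncing.
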(event EventTick
  (params (DeltaSeconds :type Float%20%28single-precision%29))
  (Utilities|FlowControl|Sequence
    (:then_0
      ;[1 1 1] Check Boulder Overlap
      (bind _returnvalue (Collision|BoxOverlapActors (+ (Transformation|GetActorLocation) "0,0.000000,25.000000") "50.000000,50.000000,50.000000" (Utilities|Array|MakeArray "ObjectTypeQuery4") "/Game/TestAssets/Blueprints/Boulder_Temp.Boulder_Temp_C" :!class /Script/Engine.KismetSystemLibrary))
      (Variables|Default|SetIsBlocked _returnvalue))
    (:then_1
      ;[1 1 1] Alternate Geyser Activity
      (if (Variables|Default|GetIsBlocked)
        (CallFunction|DisableSmoke)
        (CallFunction|DisableBouncePad)
        (else
          (bind _output_get (Variables|Default|SetCounter (+ DeltaSeconds (Variables|Default|GetCounter))))
          (Utilities|FlowControl|Sequence
            (:then_0
              (if (Math|Float|InRange(Float) _output_get 2.0 4.0 true false)
                (Components|Activation|Activate (Variables|Default|Getgeyser_small) false)
                (CallFunction|EnableBouncePad)))
            (:then_1
              (if (>= (Variables|Default|GetCounter) 4.0)
                (CallFunction|EnableSmoke)
                (CallFunction|BlockBoxUp)
                (if (>= (Variables|Default|GetCounter) 7.0)
                  (CallFunction|DisableSmoke)
                  (CallFunction|BlockBoxDown)
                  (CallFunction|DisableBouncePad)
                  (Variables|Default|SetCounter 0.0))))))))))

(event EventBeginPlay
  ;[1 1 1] Start with Geyser Off
  (CallFunction|DisableSmoke)
  (Components|Activation|Deactivate (Variables|Default|Getgeyser_small))
  (bind _returnvalue (Game|SpawnActorfromClass "/Game/TestAssets/Blueprints/BouncePad.BouncePad_C" (Math|Transform|MakeTransform "0.000000, 0,5.000000" "0, 0, 0" "1.500000,1.500000,0.050000") "Undefined" 0 0))
  (bind _output_get (Variables|Default|SetMyBouncePad _returnvalue))
  (Rendering|SetVisibility (Variables|/Script/Engine.Actor|GetRootComponent _output_get) false false)
  (Transformation|AttachActorToActor _output_get self "None" "KeepRelative" "KeepRelative" "KeepRelative" true))

(fn ConstructionScript)

(fn DisableSmoke
  (Collision|SetCollisionEnabled (Variables|Default|GetBlock_Box) "NoCollision")
  (Components|Activation|Deactivate (Variables|Default|GetGeyser_Smoke)))

(fn EnableSmoke
  (Components|Activation|Deactivate (Variables|Default|Getgeyser_small))
  (Collision|SetCollisionEnabled (Variables|Default|GetBlock_Box) "QueryAndPhysics")
  (Components|Activation|Activate (Variables|Default|GetGeyser_Smoke) false))

(fn EnableBouncePad
  (bind _asbounce_pad (Utilities|Casting|CastToBouncePad (Variables|Default|GetMyBouncePad)))
  (Variables|/Script/Engine.PrimitiveComponent|SetbGenerateOverlapEvents (Variables|/Game/TestAssets/Blueprints/BouncePad.BouncePad_C|GetCube _asbounce_pad) true))

(fn DisableBouncePad
  (bind _asbounce_pad (Utilities|Casting|CastToBouncePad (Variables|Default|GetMyBouncePad)))
  (Variables|/Script/Engine.PrimitiveComponent|SetbGenerateOverlapEvents (Variables|/Game/TestAssets/Blueprints/BouncePad.BouncePad_C|GetCube _asbounce_pad) false))

(fn BlockBoxUp
  (Transformation|SetRelativeLocation (Variables|Default|GetBlock_Box) (+ (.Location (Math|Transform|BreakTransform (Class|KismetMathLibrary|ConvertTransformtoRelative (Transformation|GetWorldTransform (Variables|Default|GetDefaultSceneRoot)) (Transformation|GetWorldTransform (Variables|Default|GetBlock_Box))))) (* (Variables|Default|GetDirection) (* (Variables|Default|GetSpeed) (Utilities|Time|GetWorldDeltaSeconds)))) false false)
  (if (>= (Variables|Default|GetCounter) 4.5)
    (Transformation|SetRelativeLocation (Variables|Default|GetBlock_Box) "0, 0, 0" false false)))

(fn BlockBoxDown
  (Transformation|SetRelativeLocation (Variables|Default|GetBlock_Box) "0, 0,-300.000000" false true))