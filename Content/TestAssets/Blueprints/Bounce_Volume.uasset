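; Bounce volume actor that launches physics objects which overlap it, likely a test asset given its folder.
; On begin overlap it waits a short delay, then casts the other actor's root to a primitive component and stops if that fails.
; It adds an impulse at that component's location, using a boulder-specific impulse for Boulder_Temp actors and the fruit impulse for everything else.
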(event Collision|EventActorBeginOverlap
  (params (OtherActor :type Actor%20Object%20Reference))
  (Utilities|FlowControl|Delay 0.25)
  (bind _asprimitive_component (Utilities|Casting|CastToPrimitiveComponent (Variables|/Script/Engine.Actor|GetRootComponent OtherActor)))
  (Utilities|Casting|CastToBoulder_Temp OtherActor
    (:then
      (Variables|Default|SetImpulse (Variables|Default|GetBoulder%20Impulse)))
    (:CastFailed
      (Variables|Default|SetImpulse (Variables|Default|GetFruit%20Impulse))))
  (Physics|AddImpulseatLocation _asprimitive_component (Variables|Default|GetImpulse) (Transformation|GetWorldLocation _asprimitive_component) "None"))

(fn ConstructionScript)