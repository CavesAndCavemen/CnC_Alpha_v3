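; CrystalBall is a physics prop that can be picked up and dropped, and acts as a level switch when hit.
; Pickup turns off the sphere's physics and attaches the root to the given component, while Drop re-enables physics and detaches, both keeping world transforms.
; Hit compares the current level name with StartupMap, opening Beta on a match and Startup_Map otherwise.
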(event Collision|EventHit
  (params (MyComp :type Primitive%20Component%20Object%20Reference) (Other :type Actor%20Object%20Reference) (OtherComp :type Primitive%20Component%20Object%20Reference) (bSelfMoved :type Boolean) (HitLocation :type Vector :default "0, 0, 0") (HitNormal :type Vector :default "0, 0, 0") (NormalImpulse :type Vector :default "0, 0, 0") (Hit :type Hit%20Result%20Structure%20%28by%20ref%29))
  ;[1 1 1] Change Level
  (bind _returnvalue (Game|GetCurrentLevelName true))
  (if (Utilities|Enum|Equal(Enum) _returnvalue (Variables|Default|GetStartupMap))
    (Game|OpenLevel(byName) "Beta")
    (else
      (Game|OpenLevel(byName) "Startup_Map"))))

(event EventPickup
  (params (Attach%20To :type Scene%20Component%20Object%20Reference))
  ;[1 1 1] Comment
  (Physics|SetSimulatePhysics (Variables|Default|GetSphere) false)
  (Transformation|AttachComponentToComponent (Variables|Transformation|GetRootComponent) Attach%20To "None" "KeepWorld" "KeepWorld" "KeepWorld" true))

(event EventDrop
  ;[1 1 1] Comment
  (Physics|SetSimulatePhysics (Variables|Default|GetSphere) true)
  (Transformation|DetachFromActor "KeepWorld" "KeepWorld" "KeepWorld"))

(fn ConstructionScript)