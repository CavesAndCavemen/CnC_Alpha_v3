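; Geyser actor that launches overlapping actors with an impulse, using a stronger-or-weaker preset for boulders versus everything else (fruit).
; Each tick a box check for Boulder_Temp physics bodies marks it blocked, switching off the smoke and BounceVolume overlap events.
; It starts off at BeginPlay, then stays active whenever unblocked.
; The timed on/off cycle is disconnected, though its counter still increments.
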(event Collision|EventActorBeginOverlap
  (params (OtherActor :type Actor%20Object%20Reference))
  ;[1 1 1] If Overlap Smoke, Add Impulse
  (bind _asprimitive_component (Utilities|Casting|CastToPrimitiveComponent (Variables|/Script/Engine.Actor|GetRootComponent OtherActor)))
  (Utilities|Casting|CastToBoulder_Temp OtherActor
    (:then
      (Variables|Default|SetImpulse (Variables|Default|GetBoulder%20Impulse)))
    (:CastFailed
      (Variables|Default|SetImpulse (Variables|Default|GetFruit%20Impulse))))
  (Physics|AddImpulseatLocation _asprimitive_component (Variables|Default|GetImpulse) (Transformation|GetWorldLocation _asprimitive_component) "None"))

(event EventTick
  (params (DeltaSeconds :type Float%20%28single-precision%29))
  (Utilities|FlowControl|Sequence
    (:then_0
      ;[1 1 1] Check Boulder Overlap
      (bind _returnvalue (Collision|BoxOverlapActors (+ (Transformation|GetActorLocation) "0,0.000000,25.000000") "50.000000,50.000000,50.000000" (Utilities|Array|MakeArray "ObjectTypeQuery4") "/Game/TestAssets/Blueprints/Boulder_Temp.Boulder_Temp_C" :!class /Script/Engine.KismetSystemLibrary))
      (Variables|Default|SetIsBlocked _returnvalue))
    (:then_1
      ;[1 1 1] Alternate Geyser Activity
      (if (Variables|Default|GetIsBlocked)
        (Components|Activation|Deactivate (Variables|Default|GetGeyser_Smoke))
        (Variables|/Script/Engine.PrimitiveComponent|SetbGenerateOverlapEvents (Variables|Default|GetBounceVolume) false)
        (else
          (Variables|Default|SetCounter (+ DeltaSeconds (Variables|Default|GetCounter)))
          (if true
            (Components|Activation|Activate (Variables|Default|GetGeyser_Smoke) false)
            (Variables|/Script/Engine.PrimitiveComponent|SetbGenerateOverlapEvents (Variables|Default|GetBounceVolume) true)))))))

(event EventBeginPlay
  ;[1 1 1] Start with Geyser Off
  (Components|Activation|Deactivate (Variables|Default|GetGeyser_Smoke))
  (Variables|/Script/Engine.PrimitiveComponent|SetbGenerateOverlapEvents (Variables|Default|GetBounceVolume) false))

(fn ConstructionScript)