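; Test actor that spawns Boulder_Temp actors when a Boulder_Temp hits it.
; On each hit it rolls a random MaxSpawns from one to three, then loops spawning boulders at the Sphere component's world location while NumberOfSpawns is at or below that limit.
; NumberOfSpawns is never reset, so later hits spawn only if their roll reaches the running count.
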(event Collision|EventHit
  (params (MyComp :type Primitive%20Component%20Object%20Reference) (Other :type Actor%20Object%20Reference) (OtherComp :type Primitive%20Component%20Object%20Reference) (bSelfMoved :type Boolean) (HitLocation :type Vector :default "0, 0, 0") (HitNormal :type Vector :default "0, 0, 0") (NormalImpulse :type Vector :default "0, 0, 0") (Hit :type Hit%20Result%20Structure%20%28by%20ref%29))
  (Utilities|Casting|CastToBoulder_Temp Other)
  (bind _output_get (Variables|Default|SetMax%20Spawns (Math|Random|RandomIntegerinRange 1 3)))
  (while (<= (Variables|Default|GetNumber%20of%20Spawns) _output_get)
    (Game|SpawnActorfromClass "/Game/TestAssets/Blueprints/Boulder_Temp.Boulder_Temp_C" (Math|Conversions|ToTransform(Vector) (Transformation|GetWorldLocation (Variables|Default|GetSphere))) "Undefined" 0 0)
    (Variables|Default|SetNumber%20of%20Spawns (+ (Variables|Default|GetNumber%20of%20Spawns) 1))))

(fn ConstructionScript)