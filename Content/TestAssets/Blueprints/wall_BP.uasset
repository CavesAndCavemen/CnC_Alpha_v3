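; Breakable wall Blueprint that shatters into flying boulders when a Boulder_Temp overlaps its Cube component.
; On overlap it destroys the wall mesh and Cube, then adds a child actor component, apparently the destructible replacement.
; It spawns a random handful of Boulder_Temp actors at random points within a wall-sized box.
; Each spawned boulder gets an impulse toward the player pawn, scaled by distance, and prints that direction vector.
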(event OnComponentBeginOverlap(Cube)
  (params (OverlappedComponent :type Primitive%20Component%20Object%20Reference) (OtherActor :type Actor%20Object%20Reference) (OtherComp :type Primitive%20Component%20Object%20Reference) (OtherBodyIndex :type Integer) (bFromSweep :type Boolean) (SweepResult :type Hit%20Result%20Structure%20%28by%20ref%29))
  (bind _self self)
  (bind _returnvalue (Transformation|GetActorTransform _self))
  (bind (_location _rotation) (Math|Transform|BreakTransform _returnvalue))
  (Utilities|Casting|CastToBoulder_Temp OtherActor)
  ;[1 1 1] Replace with Destructable
  (Components|DestroyComponent (Variables|Default|Getgeo_wall_v1))
  (Components|DestroyComponent (Variables|Default|GetCube))
  (AddComponent|AddChildActorComponent false)
  ;[1 1 1] Spawn Boulders
  (bind _output_get (Variables|Default|SetMax%20Spawns (Math|Random|RandomIntegerinRange 2 6)))
  (while (<= (Variables|Default|GetNumberOfSpawns) _output_get)
    (bind _returnvalue_2 (Game|SpawnActorfromClass "/Game/TestAssets/Blueprints/Boulder_Temp.Boulder_Temp_C" (Math|Transform|MakeTransform (Math|Random|RandomPointinBoundingBox _location (Math|Vector|MakeVector 4e+01 1.2e+02 8e+01)) _rotation) "Undefined" 0 0))
    (Variables|Default|SetNumberOfSpawns (+ (Variables|Default|GetNumberOfSpawns) 1))
    (Physics|AddImpulse (Variables|/Game/TestAssets/Blueprints/Boulder_Temp.Boulder_Temp_C|GetSphere _returnvalue_2) (* (- (Transformation|GetActorLocation (Game|Player|GetPlayerPawn 0)) (Transformation|GetWorldLocation (Variables|/Game/TestAssets/Blueprints/Boulder_Temp.Boulder_Temp_C|GetSphere _returnvalue_2))) 1.5e+03) "None" false)
    (Development|PrintString (Utilities|String|ToString(Vector) (- (Transformation|GetActorLocation (Game|Player|GetPlayerPawn 0)) (Transformation|GetWorldLocation (Variables|/Game/TestAssets/Blueprints/Boulder_Temp.Boulder_Temp_C|GetSphere _returnvalue_2)))))))

(fn ConstructionScript)