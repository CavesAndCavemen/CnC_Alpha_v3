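; VR player pawn that gives the player two motion controllers for grabbing objects and spawning crystal balls.
; On BeginPlay it sets floor-level tracking for Oculus or SteamVR headsets, then spawns left and right BP_MotionController actors attached to VrOrigin.
; Grab inputs forward grab and release to the matching controller, while either spawn input creates a CrystalBall at the CrystalBallPoint transform.
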(event EventBeginPlay
  (bind _returnvalue (Math|Transform|MakeTransform "0, 0, 0"))
  (bind _self self)
  (bind _vr_origin (Variables|Default|GetVr_Origin))
  (Utilities|FlowControl|Sequence
    (:then_0
      ;[1 1 1] Setup Player Height for Various Platforms
      (switch name (Class|HeadMountedDisplayFunctionLibrary|GetHMDDeviceName)
        (:OculusHMD
          _)
        (:Steam%20VR
          _))
      (Class|HeadMountedDisplayFunctionLibrary|SetTrackingOrigin "Floor"))
    (:then_1
      ;[1 1 1] Spawn and Attach Both MotionControllers
      (Utilities|FlowControl|Sequence
        (:then_0
          (bind _returnvalue_2 (Game|SpawnActorfromClass "/Game/TestAssets/Blueprints/BP_MotionController.BP_MotionController_C" _returnvalue "AlwaysSpawn" _self "Left" 0))
          (Variables|Default|SetLeftController _returnvalue_2)
          (Transformation|AttachComponentToComponent _returnvalue_2 _vr_origin "None" "SnapToTarget" "SnapToTarget" "KeepWorld" false))
        (:then_1
          (bind _returnvalue_3 (Game|SpawnActorfromClass "/Game/TestAssets/Blueprints/BP_MotionController.BP_MotionController_C" _returnvalue "AlwaysSpawn" _self "Right" 0))
          (Variables|Default|SetRightController _returnvalue_3)
          (Transformation|AttachComponentToComponent _returnvalue_3 _vr_origin "None" "SnapToTarget" "SnapToTarget" "KeepWorld" false))))))

(event Input|ActionEvents|InputActionGrabLeft
  (params (Key :type Key%20Structure))
  (bind _leftcontroller (Variables|Default|GetLeftController))
  ;[1 1 1] Manage Input
  (:Pressed
    (Default|GrabActor _leftcontroller))
  (:Released
    (Default|ReleaseActor _leftcontroller)))

(event Input|ActionEvents|InputActionGrabRight
  (params (Key :type Key%20Structure))
  (bind _rightcontroller (Variables|Default|GetRightController))
  ;[1 1 1] Manage Input
  (:Pressed
    (Default|GrabActor _rightcontroller))
  (:Released
    (Default|ReleaseActor _rightcontroller)))

(event Input|ActionEvents|InputActionSpawnLeft
  (params (Key :type Key%20Structure))
  ;[1 1 1] Manage Input
  (:Pressed
    (Game|SpawnActorfromClass "/Game/TestAssets/Blueprints/CrystalBall.CrystalBall_C" (Transformation|GetWorldTransform (Variables|Default|GetCrystalBallPoint)) "Undefined" 0 0)))

(event Input|ActionEvents|InputActionSpawnRight
  (params (Key :type Key%20Structure))
  ;[1 1 1] Manage Input
  (:Pressed
    (Game|SpawnActorfromClass "/Game/TestAssets/Blueprints/CrystalBall.CrystalBall_C" (Transformation|GetWorldTransform (Variables|Default|GetCrystalBallPoint)) "Undefined" 0 0)))

(fn ConstructionScript)