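; Throwable teleport fruit that moves the player, with a camera fade, to a distant BP_Floor it hits after being picked up.
; On an unforested mossy island it spawns a Tree instead and marks the island forested.
; Pickup attaches it and asks its home tree for a replacement after a delay; Drop restores physics.
; River overlaps cancel teleporting, and these or failed hits start a Tick-driven timer that destroys stray fruit.
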(event Custom|CustomEvent
  (params (DeltaSeconds :type Float%20%28single-precision%29))
  (bind _self self)
  (bind _returnvalue (Transformation|GetActorLocation _self))
  (if (Math|Vector|NotEqual(Vector) (Variables|Default|GetMidairLocation) (Transformation|GetActorLocation self) 0.1)
    (if (stale _output_get)
      (bind _output_get (Variables|Default|SetTrailCounter (+ DeltaSeconds (Variables|Default|GetTrailCounter))))
      (if (>= _output_get 0.1)
        (Effects|SpawnEmitteratLocation "/Game/TestAssets/Particles/Trail/trail_template.trail_template" _returnvalue)
        (Variables|Default|SetTrailCounter 0.0)
        (Variables|Default|SetMidairLocation _returnvalue)))
    (else
      (Variables|Default|SetInAir false))))

(event Collision|EventActorBeginOverlap
  (params (OtherActor :type Actor%20Object%20Reference))
  ;[1 1 1] If Land in River, Don't Teleport
  (Utilities|Casting|CastToRiver_Temp_BP OtherActor)
  (Variables|Default|SetIsGrabbed false)
  (Variables|Default|SetTest%20for%20Destroy true))

(event EventPickup
  (params (Attach%20To :type Scene%20Component%20Object%20Reference))
  ;[1 1 1] Pickup and Drop
  (Physics|SetSimulatePhysics (Variables|Debug|GetStaticMeshComponent) false)
  (bind _returnvalue (Transformation|AttachComponentToComponent (VehicleSound|GetRootComponent) Attach%20To "None" "KeepWorld" "KeepWorld" "KeepWorld" false))
  (Variables|Default|SetIsGrabbed _returnvalue)
  (Variables|Default|SetTest%20for%20Destroy false)
  ;[1 1 1] Spawn New Fruit
  (Utilities|FlowControl|Delay 3.0)
  (bind _astree (Utilities|Casting|CastToTree (Variables|Default|GetHomeTree)))
  (Default|FruitPicked _astree (Variables|Default|GetSpawn%20Location) self))

(event EventDrop
  ;[1 1 1] Pickup and Drop
  (Physics|SetSimulatePhysics (Variables|Debug|GetStaticMeshComponent) true)
  (Transformation|DetachFromActor "KeepWorld" "KeepWorld" "KeepWorld"))

(event Collision|EventHit
  (params (MyComp :type Primitive%20Component%20Object%20Reference) (Other :type Actor%20Object%20Reference) (OtherComp :type Primitive%20Component%20Object%20Reference) (bSelfMoved :type Boolean) (HitLocation :type Vector :default "0, 0, 0") (HitNormal :type Vector :default "0, 0, 0") (NormalImpulse :type Vector :default "0, 0, 0") (Hit :type Hit%20Result%20Structure%20%28by%20ref%29))
  ;[1 1 1] Teleport Player
  (if (Variables|Default|GetIsGrabbed)
    (bind _asbp_floor (Utilities|Casting|CastToBP_Floor Other)
      (:then
        (if (Math|Vector|NotEqual(Vector) (Transformation|GetActorLocation _asbp_floor) (Transformation|GetActorLocation (Game|Player|GetPlayerPawn 0)) 1.5e+02)
          (bind _asbp_mossy_island (Utilities|Casting|CastToBP_MossyIsland _asbp_floor)
            (:then
              (if (Variables|/Game/TestAssets/Blueprints/BP_MossyIsland.BP_MossyIsland_C|GetIsForested _asbp_mossy_island)
                (CameraFades|StartCameraFade :self (Game|GetPlayerCameraManager 0) :ToAlpha 1.0 :Duration 0.5 :!label _label)
                (Transformation|Teleport (Game|Player|GetPlayerPawn 0) (Transformation|GetWorldLocation (Variables|/Game/TestAssets/Blueprints/BP_Floor.BP_Floor_C|GetScene _asbp_floor)) "0, 0, 0")
                (CameraFades|StartCameraFade :self (Game|GetPlayerCameraManager 0) :FromAlpha 1.0 :Duration 0.5)
                (Utilities|FlowControl|Delay 0.05)
                (Actor|DestroyActor)
                (else
                  ;[1 1 1] With First Fruit Hit, Spawn Tree
                  (Game|SpawnActorfromClass "/Game/TestAssets/Blueprints/Tree.Tree_C" (Math|Transform|MakeTransform HitLocation) "Undefined" 0 0)
                  (Variables|/Game/TestAssets/Blueprints/BP_MossyIsland.BP_MossyIsland_C|SetIsForested _asbp_mossy_island true)
                  (Actor|DestroyActor))))
            (:CastFailed
              (goto _label)))
          (else
            (Variables|Default|SetTest%20for%20Destroy true))))
      (:CastFailed
        (Variables|Default|SetTest%20for%20Destroy true)))
    (else
      (Variables|Default|SetTest%20for%20Destroy true))))

(event EventTick
  (params (DeltaSeconds :type Float%20%28single-precision%29))
  ;[1 1 1] Destroy if Unnecessary
  (if (Variables|Default|GetTest%20for%20Destroy)
    (Development|PrintString "Test for Destroy")
    (bind _output_get (Variables|Default|SetDestructionCounter (+ DeltaSeconds (Variables|Default|GetDestructionCounter))))
    (if (Math|Boolean|ANDBoolean (>= _output_get 2e+01) (Physics|IsSimulatingPhysics (Variables|Debug|GetStaticMeshComponent) "None") (Math|Vector|NotEqual(Vector) (Transformation|GetActorLocation) (Transformation|GetActorLocation (Game|Player|GetPlayerPawn 0)) 1.5e+02))
      (Development|PrintString "DESTROYED")
      (Actor|DestroyActor))))

(fn ConstructionScript)